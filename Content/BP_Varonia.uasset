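; Bridge actor linking a VR game to the Varonia back office over MQTT, reporting session state and receiving start commands.
; After a short delay on BeginPlay it pings its soft state every second, subscribes to its per-client topic and fires start events with or without tutorial, guarded against repeats.
; Helpers publish party started/closed, sync player transform from the spatial config, draw colored spline-mesh boundaries and scale camera offset.
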(event Custom|OnStartWithTuto_
  ;[0.15 0.15 0.15 0.5] OnStartWithTuto
  (Development|PrintString "Start WithTuto" true true "(R=0.000000,G=1.000000,B=0.368498,A=1.000000)")
  (Default|CallOnStartwithTuto))

(event Custom|OnStartWithoutTuto_
  ;[0.15 0.15 0.15 0.5] OnStartWithoutTuto
  (Development|PrintString "Start Without Tuto" true true "(R=0.000000,G=1.000000,B=0.329391,A=1.000000)")
  (Default|CallOnStartWithoutTuto))

(event Custom|Start%20Game%20Logic
  ;[0.02141 0.15 0.01492 0.5] Listener Topic Start Game
  (Class|MqttClientBase|SetonMessageHandler (.AsMqtt%20Client%20Base (Utilities|Casting|CastToMqttClientBase (Variables|Default|GetMqttClientInterface))) (delegate Custom|On%20Message)))

(event Custom|On%20Message
  (params (message :type Mqtt%20Message%20Structure))
  (bind _message (Utilities|Struct|BreakMqttMessage message))
  ;[0.02141 0.15 0.01492 0.5] Listener Topic Start Game
  (Utilities|FlowControl|Sequence
    (:then_0
      (if (Utilities|String|Contains _message "GET_SOFTPARTYSKIPTUTOANDSTART_RESULT")
        (if (Variables|/Script/VaroniaBackOffice.VaroniaBackOfficeManager|GetGameStarted (Subsystems|GetVaroniaBackOfficeManager))
          (Development|PrintString "Game Already Started" true true "(R=1.000000,G=0.000000,B=0.127360,A=1.000000)" :!label _label)
          (else
            (CallFunction|OnStartWithoutTuto)
            (Variables|/Script/VaroniaBackOffice.VaroniaBackOfficeManager|SetGameStarted (Subsystems|GetVaroniaBackOfficeManager) true :!label _label_2)))))
    (:then_1
      (if (Utilities|String|Contains _message "GET_SOFTPARTYSTART_RESULT")
        (if (Variables|/Script/VaroniaBackOffice.VaroniaBackOfficeManager|GetGameStarted (Subsystems|GetVaroniaBackOfficeManager))
          (goto _label)
          (else
            (CallFunction|OnStartwithTuto)
            (goto _label_2)))))))

(event Custom|Ping
  ;[0.15 0.01041 0.1299 0.5] Ping  (send every second )
  (Utilities|FlowControl|Delay 1.0 :!label _label)
  (CallFunction|SetSoftState (Variables|/Script/VaroniaBackOffice.VaroniaBackOfficeManager|GetCurrentSoftState (Subsystems|GetVaroniaBackOfficeManager)))
  (goto _label))

(event EventBeginPlay
  (bind _returnvalue (Subsystems|GetVaroniaBackOfficeManager))
  (bind _mqtthandler (Variables|/Script/VaroniaBackOffice.VaroniaBackOfficeManager|GetMqttHandler _returnvalue))
  (Utilities|FlowControl|Sequence
    (:then_0
      (Utilities|FlowControl|Delay 0.5) ; Max Delay to connect MQTT server
      (if (Class|VaroniaMqttClient|IsConnected _mqtthandler) ; Check MQTT Connection
        (CallFunction|Ping) ; Lanch  "Ping" Loop
        (CallFunction|SubscribeTopic) ; Subscribe to 'ServerToUnity'
        (CallFunction|StartGameLogic) ; Listener 'ServerToUnity'
        (Default|CallBackOfficeIsReady) ; VARONIA BACK OFFICE IS READY
        (else
          (Development|PrintString "MQTT No Connected" true true "(R=1.000000,G=0.000000,B=0.007738,A=1.000000)"))))
    (:then_1
      (Variables|Default|SetMqttClientInterface (Class|VaroniaMqttClient|GetMqttClient _mqtthandler)))))

(fn ConstructionScript)

(fn SetSoftState
  (params (New%20State :type ESoftState%20Enum :default "UNKNOWN"))
  (bind _returnvalue (Math|Conversions|ToInteger(Byte) New%20State))
  (bind _returnvalue_2 (Subsystems|GetVaroniaBackOfficeManager))
  (bind _mqtthandler (Variables|/Script/VaroniaBackOffice.VaroniaBackOfficeManager|GetMqttHandler _returnvalue_2))
  (bind _clientid (Variables|/Script/VaroniaBackOffice.VaroniaMqttClient|GetClientID _mqtthandler))
  (bind _returnvalue_3 (Class|VaroniaMqttLibrary|FormatMqttMessage _clientid "SET_SOFTSTATE" _returnvalue))
  ;[0.1142 0.15 0.04626 0.5] SetSoftState
  (Variables|/Script/VaroniaBackOffice.VaroniaBackOfficeManager|SetCurrentSoftState _returnvalue_2 New%20State)
  (if (Class|VaroniaMqttClient|IsConnected _mqtthandler)
    (bind _topicandclientid (CallFunction|SetTopic "UnityToServer"))
    (Class|MqttClientInterface|Publish (Class|VaroniaMqttClient|GetMqttClient _mqtthandler) (Utilities|Struct|MakeMqttMessage _returnvalue_3 0 _topicandclientid))
    (return _returnvalue_3)))

(fn SetTopic
  (params (Topic :type String))
  (return (Utilities|String|Append Topic "/" (Utilities|String|ToString(Integer) (Variables|/Script/VaroniaBackOffice.VaroniaMqttClient|GetClientID (Variables|/Script/VaroniaBackOffice.VaroniaBackOfficeManager|GetMqttHandler (Subsystems|GetVaroniaBackOfficeManager)))))))

(fn SubscribeTopic
  (if (Class|VaroniaMqttClient|IsConnected (Variables|/Script/VaroniaBackOffice.VaroniaBackOfficeManager|GetMqttHandler (Subsystems|GetVaroniaBackOfficeManager)))
    (bind _topicandclientid (CallFunction|SetTopic "ServerToUnity"))
    (Class|MqttClientBase|Subscribe (.AsMqtt%20Client%20Base (Utilities|Casting|CastToMqttClientBase (Variables|Default|GetMqttClientInterface))) _topicandclientid)))

(fn SetSoftPartyStarted
  (bind _returnvalue (Subsystems|GetVaroniaBackOfficeManager))
  (bind _mqtthandler (Variables|/Script/VaroniaBackOffice.VaroniaBackOfficeManager|GetMqttHandler _returnvalue))
  (bind _clientid (Variables|/Script/VaroniaBackOffice.VaroniaMqttClient|GetClientID _mqtthandler))
  (bind _returnvalue_2 (Class|VaroniaMqttLibrary|FormatMqttMessage _clientid "SET_SOFTPARTYSTARTED" -1))
  ;[0.5679 0.631 1 0.5] SetSoftPartyStarted
  (if (Class|VaroniaMqttClient|IsConnected _mqtthandler)
    (bind _topicandclientid (CallFunction|SetTopic "UnityToServer"))
    (Class|MqttClientInterface|Publish (Class|VaroniaMqttClient|GetMqttClient _mqtthandler) (Utilities|Struct|MakeMqttMessage _returnvalue_2 0 _topicandclientid))
    (return _returnvalue_2)))

(fn SetSoftPartyClosed
  (bind _returnvalue (Subsystems|GetVaroniaBackOfficeManager))
  (bind _mqtthandler (Variables|/Script/VaroniaBackOffice.VaroniaBackOfficeManager|GetMqttHandler _returnvalue))
  (bind _clientid (Variables|/Script/VaroniaBackOffice.VaroniaMqttClient|GetClientID _mqtthandler))
  (bind _returnvalue_2 (Class|VaroniaMqttLibrary|FormatMqttMessage _clientid "SET_SOFTPARTYCLOSED" -1))
  ;[0.5679 0.631 1 0.5] SetSoftPartyStarted
  (if (Class|VaroniaMqttClient|IsConnected _mqtthandler)
    (bind _topicandclientid (CallFunction|SetTopic "UnityToServer"))
    (Class|MqttClientInterface|Publish (Class|VaroniaMqttClient|GetMqttClient _mqtthandler) (Utilities|Struct|MakeMqttMessage _returnvalue_2 0 _topicandclientid))
    (return _returnvalue_2)))

(fn SyncPosandRot
  (params (PlayerVR :type Actor%20Object%20Reference))
  (bind _returnvalue (Subsystems|GetVaroniaBackOfficeManager))
  (bind _spatialconfig (Variables|/Script/VaroniaBackOffice.VaroniaBackOfficeManager|GetSpatialConfig _returnvalue))
  (bind (_id _name _areavalue _maxrect _groupname _maxplayer _syncposition _syncrotation) (Utilities|Struct|BreakSpatialConfig _spatialconfig))
  ;[0.6719 7.9e-05 0.00138 0.5] Sync Position
  (Transformation|SetActorLocation PlayerVR _syncposition false false)
  (Transformation|SetActorRotation PlayerVR _syncrotation))

(fn SpawnBoundaries
  (params (PlayerVR :type Actor%20Object%20Reference))
  ;[1 0.2164 0.004845 0.5] Spawn Boundaries
  (for _array_element (.boundaries (Variables|/Script/VaroniaBackOffice.VaroniaBackOfficeManager|GetSpatialConfig (Subsystems|GetVaroniaBackOfficeManager)))
    ;[0.15 0.15 0.15 0.5] Spawn Boundary
    (bind _returnvalue (AddComponent|AddSplineComponent PlayerVR false))
    (bind _output_get (LocalVariables|Set_CurrentSpine _returnvalue))
    (LocalVariables|Set_CurrentColor (.BoundaryColor (Utilities|Struct|BreakSpatialBoundary _array_element)))
    (Spline|ClearSplinePoints _output_get true)
    (for (_array_element_2 _array_index) (.Points (Utilities|Struct|BreakSpatialBoundary _array_element))
      (Spline|AddSplinePoint (LocalVariables|Get_CurrentSpine) _array_element_2 "Local" true)
      (Spline|SetSplinePointType (LocalVariables|Get_CurrentSpine) _array_index "Linear" true))
    (Spline|SetClosedLoop (LocalVariables|Get_CurrentSpine) true true)
    (for _index (range 0 _array_index)
      (bind _returnvalue_2 (AddComponent|AddSplineMeshComponent PlayerVR false))
      (LocalVariables|Set_CurrentSplineMesh _returnvalue_2)
      (bind _returnvalue_3 (Rendering|Material|CreateDynamicMaterialInstance "/VaroniaBackOffice/M_LINE.M_LINE" "" "None" :!class /Script/Engine.KismetMaterialLibrary))
      (Rendering|Material|SetVectorParameterValue _returnvalue_3 "BaseColor" (LocalVariables|Get_CurrentColor) :!class /Script/Engine.MaterialInstanceDynamic)
      (Rendering|Material|SetMaterial (LocalVariables|Get_CurrentSplineMesh) 0 _returnvalue_3)
      (bind _returnvalue_4 (AddComponent|AddStaticMeshComponent PlayerVR false))
      (Rendering|Material|SetMaterial _returnvalue_4 0 _returnvalue_3)
      (Transformation|SetRelativeLocation _returnvalue_4 (Spline|GetLocationatSplinePoint (LocalVariables|Get_CurrentSpine) _index "Local") false false)
      (SplineMesh|SetStartandEnd (LocalVariables|Get_CurrentSplineMesh) (Spline|GetLocationatSplinePoint (LocalVariables|Get_CurrentSpine) _index "Local") (- (Spline|GetLocationatSplinePoint (LocalVariables|Get_CurrentSpine) (+ _index 1) "Local") (Spline|GetLocationatSplinePoint (LocalVariables|Get_CurrentSpine) _index "Local")) (Spline|GetLocationatSplinePoint (LocalVariables|Get_CurrentSpine) (+ _index 1) "Local") (- (Spline|GetLocationatSplinePoint (LocalVariables|Get_CurrentSpine) (+ _index 1) "Local") (Spline|GetLocationatSplinePoint (LocalVariables|Get_CurrentSpine) _index "Local")) false :!class /Script/Engine.SplineMeshComponent))))

(fn CoefMul
  (params (PosMul :type Scene%20Component%20Object%20Reference) (Camera :type Camera%20Component%20Object%20Reference))
  (bind _returnvalue (Subsystems|GetVaroniaBackOfficeManager))
  (bind _relativelocation (Variables|/Script/Engine.SceneComponent|GetRelativeLocation Camera))
  (bind _spatialconfig (Variables|/Script/VaroniaBackOffice.VaroniaBackOfficeManager|GetSpatialConfig _returnvalue))
  ;[0.21 0.4081 0.8958 0.5] Apply Multiplicator
  (Transformation|SetRelativeLocation PosMul (Math|Vector|MakeVector (* (.x _relativelocation) (.multiplier _spatialconfig)) (* (.y _relativelocation) (.multiplier _spatialconfig)) 0.0) false false))

(fn SetSync
  (params (PlayerVR :type Actor%20Object%20Reference))
  ;[0.2031 0.08463 0.08544 0.5] Varonia Sync
  (CallFunction|SyncPosandRot PlayerVR)
  (CallFunction|SpawnBoundaries PlayerVR))